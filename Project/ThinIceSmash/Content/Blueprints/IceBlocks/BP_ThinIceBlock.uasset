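; Thin ice block actor that shatters with a sound when its Break event is called.
; Construction applies the ice material to the root mesh, and BeginPlay stores a dynamic instance of it.
; Break reveals a destructible component, shatters it with radial damage and impulse from its own location, then hides the intact mesh.
; An opacity change and a directional-damage alternative remain as unconnected nodes.
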(event `self.ReceiveBeginPlay`
  (`parent.ReceiveBeginPlay`)
  (bind _returnvalue (`PrimitiveComponent.CreateDynamicMaterialInstance` (`self.m_Root`) 0 "/Game/Materials/M_Ice.M_Ice"))
  (set `self.ThinIce` _returnvalue))

(event `self.Break`
  (params (actor :type "Actor Object Reference"))
  (`GameplayStatics.PlaySound2D` (`self.BreakSFX`))
  (`SceneComponent.SetVisibility` (`self.Destructible`) true false)
  (`DestructibleComponent.ApplyRadiusDamage` (`self.Destructible`) 300.0 (`SceneComponent.K2_GetComponentLocation` (`self.Destructible`)) 800.0 5000.0 true)
  (`SceneComponent.SetVisibility` (`self.m_Root`) false false))

(fn `UserConstructionScript`
  (`PrimitiveComponent.SetMaterial` (`self.m_Root`) 0 "/Game/Materials/M_Ice.M_Ice"))